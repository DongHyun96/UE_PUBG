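; Inventory component for BPC_Player that handles backpack pickup and the equipment panel.
; IA_F sphere-traces forward from the player camera, appends a hit BP_BackPack's ItemData to BackPackSlot and destroys that actor.
; IA_I toggles WB_Equipment_UI, creating it on first use and then reusing it through visibility changes, with InitUI on each open.
; An open panel shows the cursor, switches input to game-and-UI and disables character movement; closing restores walking.
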(event Input|EnhancedActionEvents|EnhancedInputActionIA_I
  (params (ActionValue :type Boolean) (ElapsedSeconds :type Float%20%28double-precision%29) (TriggeredSeconds :type Float%20%28double-precision%29) (InputAction :type Input%20Action%20Object%20Reference :default "/Game/Project_PUBG/Common/Character/Input/IA_I.IA_I"))
  (bind _returnvalue (Game|GetPlayerController 0))
  ;[1 1 1] InvenSystem Panel
  (:Started
    (if (not (Variables|Default|GetIsPanelOpend))
      (Variables|Default|SetIsPanelOpend true)
      (bind _equipment_widget (Variables|Default|GetEquipment%20Widget)
        (:then
          (Widget|SetVisibility _equipment_widget "Visible")
          (Default|InitUI (Variables|Default|GetEquipment%20Widget)))
        (:else
          (bind _returnvalue_2 (UserInterface|CreateWidget "/Game/Project_PUBG/Common/InventoryUI/Blueprint_UI/WB_Equipment_UI.WB_Equipment_UI_C"))
          (bind _output_get (Variables|Default|SetEquipment%20Widget _returnvalue_2))
          (Default|InitUI _output_get)
          (UserInterface|Viewport|AddtoViewport _output_get 0)))
      (Variables|/Script/Engine.PlayerController|SetbShowMouseCursor _returnvalue true)
      (Input|SetInputModeGameandUI _returnvalue (Variables|Default|GetEquipment%20Widget) "DoNotLock" true false)
      (bind _asbpc_player (Utilities|Casting|CastToBPC_Player (Components|GetOwner)))
      (Pawn|Components|CharacterMovement|SetMovementMode (Variables|/Script/Engine.Character|GetCharacterMovement _asbpc_player) "MOVE_None" 0)
      (else
        (Variables|Default|SetIsPanelOpend false)
        (bind _equipment_widget_2 (Variables|Default|GetEquipment%20Widget)
          (:then
            (Widget|SetVisibility _equipment_widget_2 "Hidden")
            (Variables|/Script/Engine.PlayerController|SetbShowMouseCursor _returnvalue false)
            (Input|SetInputModeGameOnly _returnvalue false)
            (bind _asbpc_player_2 (Utilities|Casting|CastToBPC_Player (Components|GetOwner)))
            (Pawn|Components|CharacterMovement|SetMovementMode (Variables|/Script/Engine.Character|GetCharacterMovement _asbpc_player_2) "MOVE_Walking" 0))
          (:else))))))

(event Input|EnhancedActionEvents|EnhancedInputActionIA_F
  (params (ActionValue :type Boolean) (ElapsedSeconds :type Float%20%28double-precision%29) (TriggeredSeconds :type Float%20%28double-precision%29) (InputAction :type Input%20Action%20Object%20Reference :default "/Game/Project_PUBG/Common/Character/Input/IA_F.IA_F"))
  (bind _follow_camera (Variables|Default|GetFollow%20Camera))
  (bind _returnvalue (Transformation|GetWorldLocation _follow_camera))
  (bind _outhit (Collision|SphereTraceForObjects _returnvalue (+ _returnvalue (* (Math|Vector|GetForwardVector (Transformation|GetWorldRotation _follow_camera)) 1000)) 15.0 (Utilities|Array|MakeArray "ObjectTypeQuery2") false 0 "ForDuration"))
  (if true
    (bind _asbp_back_pack (Utilities|Casting|CastToBP_BackPack (.HitActor (Collision|BreakHitResult _outhit))))
    (CallFunction|AddBackPack (Variables|/Game/Project_PUBG/Common/InventoryUI/Blueprint_UI/Test/BP_BackPack.BP_BackPack_C|GetItem%20Data _asbp_back_pack))
    (Actor|DestroyActor _asbp_back_pack)
    (Development|PrintString "Get item")))

(event EventBeginPlay
  (bind _asbpc_player (Utilities|Casting|CastToBPC_Player (Components|GetOwner)))
  (Variables|Default|SetFollow%20Camera (Variables|/Game/Project_PUBG/Common/Character/BPC_Player.BPC_Player_C|GetCamera _asbpc_player)))

(fn AddBackPack
  (params (NewBackPack :type S%20Slots%20Structure%20%28by%20ref%29))
  (Utilities|Array|Add (Variables|Default|GetBackPackSlot) NewBackPack))