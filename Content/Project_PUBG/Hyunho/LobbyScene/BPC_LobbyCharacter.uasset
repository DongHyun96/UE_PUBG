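; Lobby character Blueprint that displays the player's nickname on a name tag in the lobby scene.
; InitNameTag unhides the NameTagWidget component, then copies PlayerNickName from C_GameInstance into the NameTag text of its WBP_LobbyNameTag widget.
; The event graph and construction script hold only empty stubs, and nothing in this Blueprint calls InitNameTag.
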(event Custom|TempAction)

(event EventBeginPlay)

(event Collision|EventActorBeginOverlap
  (params (OtherActor :type Actor%20Object%20Reference)))

(event EventTick
  (params (DeltaSeconds :type Float%20%28single-precision%29)))

(fn ConstructionScript)

(fn InitNameTag
  (Development|SetHiddeninGame (Variables|Default|GetNameTagWidget) false false)
  (bind _asc_game_instance (Utilities|Casting|CastToC_GameInstance (Game|GetGameInstance)))
  (bind _aswbp_lobby_name_tag (Utilities|Casting|CastToWBP_LobbyNameTag (UserInterface|GetWidget (Variables|Default|GetNameTagWidget))))
  (Variables|/Script/UMG.TextBlock|SetText (Variables|/Game/Project_PUBG/DongHyun/LobbyMap/WBP_LobbyNameTag.WBP_LobbyNameTag_C|GetNameTag _aswbp_lobby_name_tag) (Utilities|Text|ToText(String) (Variables|/Script/UE_PUBG.C_GameInstance|GetPlayerNickName _asc_game_instance))))