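; Lobby scene pawn that shows the lobby and map-select widgets and loads the chosen level.
; BeginPlay adds both component-held widgets to the viewport, and StartLoading routes the selection to one of three loading macros.
; Each shows the loading widget, removes the lobby, waits briefly, then opens a LevelNames entry; only the third sets UI-only input.
; The "random" option always yields the first level, and the progress-bar and input-mapping logic are disconnected.
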(event Custom|StartLoading
  (params (SelectedNum :type Integer))
  (Variables|Default|SetIsLoading true)
  (switch int SelectedNum
    (:0
      (|LoadingAndOpenLevel))
    (:1
      (|LoadingAndOpenLevel_2))
    (:2
      (|LoadingAndOpenLevel_3))))

(event EventBeginPlay
  (UserInterface|Viewport|AddtoViewport (UserInterface|GetWidget (Variables|Default|GetLobbyUI)) 0)
  (UserInterface|Viewport|AddtoViewport (UserInterface|GetWidget (Variables|Default|GetSelectMapUI)) 0))

(event Collision|EventActorBeginOverlap
  (params (OtherActor :type Actor%20Object%20Reference)))

(event EventTick
  (params (DeltaSeconds :type Float%20%28single-precision%29)))

(fn ConstructionScript)