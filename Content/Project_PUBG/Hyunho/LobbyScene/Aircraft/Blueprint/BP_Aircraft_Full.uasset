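; Lobby scene aircraft that animates a door opening and then hands off to the lobby pawn to start loading.
; OpenTheDoor sets a flag, and Tick eases two mesh components' pitch downward with a delta-time Lerp.
; Near the target angle, it stops and calls StartLoading on BPC_LobbyScenePawn, passing Lobby_UI's SelectedNumber, or zero if the cast fails.
; A stream-level load of Shanty_Town_Map is present but never runs.
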(event Custom|OpenTheDoor
  (Variables|Default|SetIsOpening true))

(event EventBeginPlay
  (Variables|Default|SetIsLoading false))

(event Collision|EventActorBeginOverlap
  (params (OtherActor :type Actor%20Object%20Reference)))

(event EventTick
  (params (DeltaSeconds :type Float%20%28single-precision%29))
  (if (Variables|Default|GetIsOpening)
    (Variables|Default|SetAngle (Math|Float|Lerp (Variables|Default|GetAngle) -2e+01 (Utilities|Time|GetWorldDeltaSeconds)))
    (Transformation|SetRelativeRotation (Variables|Default|GetStaticMeshComponent1) (Math|Rotator|MakeRotator 0.0 (Variables|Default|GetAngle) 0.0) false false)
    (Transformation|SetRelativeRotation (Variables|Default|GetStaticMeshComponent0) (Math|Rotator|MakeRotator 0.0 (Variables|Default|GetAngle) 0.0) false false)
    (if (<= (Variables|Default|GetAngle) -19.5)
      (Variables|Default|SetIsOpening false)
      (Variables|Default|SetIsLoading true)
      (bind _foundwidgets (Widget|GetAllWidgetsOfClass "/Game/Project_PUBG/Hyunho/LobbyScene/Lobby_UI.Lobby_UI_C" true))
      (bind _aslobby_ui (Utilities|Casting|CastToLobby_UI (Utilities|Array|Get(acopy) _foundwidgets))
        (:then
          (bind _outactors (Actor|GetAllActorsOfClass "/Game/Project_PUBG/Hyunho/LobbyScene/BPC_LobbyScenePawn.BPC_LobbyScenePawn_C"))
          (Default|StartLoading (Utilities|Array|Get(acopy) _outactors) (Variables|/Game/Project_PUBG/Hyunho/LobbyScene/Lobby_UI.Lobby_UI_C|GetSelectedNumber _aslobby_ui)))
        (:CastFailed
          (bind _outactors_2 (Actor|GetAllActorsOfClass "/Game/Project_PUBG/Hyunho/LobbyScene/BPC_LobbyScenePawn.BPC_LobbyScenePawn_C"))
          (Default|StartLoading (Utilities|Array|Get(acopy) _outactors_2)))))))

(fn ConstructionScript)