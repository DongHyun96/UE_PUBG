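; Projectile bullet actor that ignores its owner while moving and leaves an oriented decal where it stops.
; On projectile stop it plays the impact sound, turns off the trail, calls DeactivateInstance and spawns BPC_Bullet_Decal, with debug prints of the hit actor.
; The decal aligns to the surface normal, rolls along the offset from LineTraceHitLocation, and stretches with that distance on shallow-angle hits.
; Upward-facing surfaces use a separate reference axis and swapped stretch axes.
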(event OnComponentBeginOverlap(Sphere)
  (params (OverlappedComponent :type Primitive%20Component%20Object%20Reference) (OtherActor :type Actor%20Object%20Reference) (OtherComp :type Primitive%20Component%20Object%20Reference) (OtherBodyIndex :type Integer) (bFromSweep :type Boolean) (SweepResult :type Hit%20Result%20Structure%20%28by%20ref%29)))

(event OnProjectileStop(BulletProjectileMovement)
  (params (ImpactResult :type Hit%20Result%20Structure%20%28by%20ref%29))
  (bind (_bblockinghit _binitialoverlap _time _distance _location _impactpoint _normal _impactnormal _physmat _hitactor _hitcomponent _hitbonename _bonename _hititem _elementindex _faceindex _tracestart _traceend) (Collision|BreakHitResult ImpactResult))
  (bind _linetracehitlocation (Variables|Default|GetLineTraceHitLocation))
  (bind _returnvalue (Math|Rotator|MakeRotfromX _impactnormal))
  (bind _returnvalue_2 (- _location _linetracehitlocation))
  (bind _returnvalue_3 (Math|Vector|VectorLength _returnvalue_2))
  (bind _returnvalue_4 (Math|Vector|Normalize _returnvalue_2))
  (Class|CBullet|PlaySound ImpactResult)
  (Components|Activation|Deactivate (Variables|Default|GetTrail))
  (Development|PrintString (Utilities|GetObjectName _hitactor))
  (Variables|Default|SetTraceVector (- _tracestart _traceend))
  (Variables|Default|SetImpact%20Normal _impactnormal)
  (Class|CBullet|DeactivateInstance)
  (if (== (Math|Vector|DotProduct (Variables|Default|GetImpact%20Normal) "0.000000,0.000000,1.000000") 1.0)
    (Variables|Default|SetPlaneVector (Math|Vector|CrossProduct (Variables|Default|GetImpact%20Normal) "0.000000,1.000000,0.000000"))
    (Game|SpawnActorfromClass "/Game/Project_PUBG/Common/Weapon/GunWeapon/BulletDecal/BPC_Bullet_Decal.BPC_Bullet_Decal_C" (Math|Transform|MakeTransform _location (Math|Rotator|MakeRotator (+ (.roll _returnvalue) (* (Math|Trig|RadiansToDegrees (Math|Trig|Acos(Degrees) (Math|Vector|DotProduct _returnvalue_4 (Variables|Default|GetPlaneVector)))) (/ (Math|Vector|DotProduct _impactnormal (Math|Vector|CrossProduct _returnvalue_4 (Variables|Default|GetPlaneVector))) (Math|Float|Absolute(Float) (Math|Vector|DotProduct _impactnormal (Math|Vector|CrossProduct _returnvalue_4 (Variables|Default|GetPlaneVector))))))) (.pitch _returnvalue) (.yaw _returnvalue)) (Math|Vector|MakeVector 5.0 (/ 1.0 (select (or (<= _returnvalue_3 1e+01) (> (Math|Vector|DotProduct (Variables|Default|GetImpact%20Normal) (Math|Vector|Normalize (Variables|Default|GetTraceVector))) 0.707107)) 1.0 (Math|Float|Min(Float) (/ _returnvalue_3 4.0) 8.0))) (select (or (<= _returnvalue_3 1e+01) (> (Math|Vector|DotProduct (Variables|Default|GetImpact%20Normal) (Math|Vector|Normalize (Variables|Default|GetTraceVector))) 0.707107)) 1.0 (Math|Float|Min(Float) (/ _returnvalue_3 4.0) 8.0)))) "Undefined" "MultiplyWithRoot" 0 0)
    (else
      (Variables|Default|SetPlaneVector (Math|Vector|CrossProduct "0.000000,0.000000,1.000000" (Variables|Default|GetImpact%20Normal)))
      (Game|SpawnActorfromClass "/Game/Project_PUBG/Common/Weapon/GunWeapon/BulletDecal/BPC_Bullet_Decal.BPC_Bullet_Decal_C" (Math|Transform|MakeTransform _location (Math|Rotator|MakeRotator (+ (.roll _returnvalue) (* (Math|Trig|RadiansToDegrees (Math|Trig|Acos(Degrees) (Math|Vector|DotProduct _returnvalue_4 (Variables|Default|GetPlaneVector)))) (/ (Math|Vector|DotProduct _impactnormal (Math|Vector|CrossProduct _returnvalue_4 (Variables|Default|GetPlaneVector))) (Math|Float|Absolute(Float) (Math|Vector|DotProduct _impactnormal (Math|Vector|CrossProduct _returnvalue_4 (Variables|Default|GetPlaneVector))))))) (.pitch _returnvalue) (.yaw _returnvalue)) (Math|Vector|MakeVector 5.0 (select (or (<= _returnvalue_3 1e+01) (> (Math|Vector|DotProduct (Variables|Default|GetImpact%20Normal) (Math|Vector|Normalize (Variables|Default|GetTraceVector))) 0.707107)) 1.0 (Math|Float|Min(Float) (/ _returnvalue_3 4.0) 8.0)) (/ 1.0 (select (or (<= _returnvalue_3 1e+01) (> (Math|Vector|DotProduct (Variables|Default|GetImpact%20Normal) (Math|Vector|Normalize (Variables|Default|GetTraceVector))) 0.707107)) 1.0 (Math|Float|Min(Float) (/ _returnvalue_3 4.0) 8.0))))) "Undefined" "MultiplyWithRoot" 0 0)))
  (Development|PrintString (Utilities|GetDisplayName _hitactor)))

(event OnComponentActivated(Sphere)
  (params (Component :type Actor%20Component%20Object%20Reference) (bReset :type Boolean)))

(event EventBeginPlay
  (Collision|IgnoreActorwhenMoving (Variables|Components|GetSphere) (Components|GetOwner) true)
  (Components|Activation|Deactivate (Variables|Default|GetTrail)))

(event Collision|EventActorBeginOverlap
  (params (OtherActor :type Actor%20Object%20Reference)))

(event EventTick
  (params (DeltaSeconds :type Float%20%28single-precision%29)))

(fn ConstructionScript)