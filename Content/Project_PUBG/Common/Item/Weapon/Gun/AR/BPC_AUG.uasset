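; AUG assault rifle weapon Blueprint in the PUBG-style project's gun item set.
; At BeginPlay it only deactivates its aim Camera, and GetLeftHandSocket returns without computing a socket from the character mesh.
; Disconnected leftover nodes hold an aim-widget visibility check using a short camera-forward line trace, a DT_Item row lookup for the AUG, and widget viewport setup, none of which run.
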(event EventBeginPlay
  (Components|Activation|SetActive (Variables|Default|GetCamera) false false))

(event Collision|EventActorBeginOverlap
  (params (OtherActor :type Actor%20Object%20Reference)))

(event EventTick
  (params (DeltaSeconds :type Float%20%28single-precision%29)))

(fn ConstructionScript)

(fn GetLeftHandSocket
  (params (CharacterMesh :type Skinned%20Mesh%20Component%20Object%20Reference))
  (return ""))