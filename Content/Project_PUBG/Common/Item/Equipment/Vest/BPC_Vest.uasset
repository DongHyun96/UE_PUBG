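; BPC_Vest is an armor vest equipment item with three levels.
; On BeginPlay it switches on ItemLevel to set the matching ItemCode string and swap the static mesh to that level's vest model.
; The construction script, overlap and tick events are empty, and a SetActorScale3D call is left unconnected.
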(event EventBeginPlay
  (Class|CVest|InitVestDatasandStaticMesh))

(event Collision|EventActorBeginOverlap
  (params (OtherActor :type Actor%20Object%20Reference)))

(event EventTick
  (params (DeltaSeconds :type Float%20%28single-precision%29)))

(event EventInitVestDatasandStaticMesh
  (bind _staticmesh (Variables|Default|GetStaticMesh))
  (switch Utilities|FlowControl|Switch|SwitchonEEquipableItemLevel (Variables|Default|GetItemLevel)
    (:LV1
      (Variables|Default|SetItemCode "Item_Armor_E_01_Lv1_C")
      (Components|StaticMesh|SetStaticMesh _staticmesh "/Game/Vest/LV1/combat-vest/source/PlateCarrierSketchfab/Combat1_Vest_LV1.Combat1_Vest_LV1"))
    (:LV2
      (Variables|Default|SetItemCode "Item_Armor_D_01_Lv2_C")
      (Components|StaticMesh|SetStaticMesh _staticmesh "/Game/Vest/LV2/VestLV2_100_1_armor_vest.VestLV2_100_1_armor_vest"))
    (:LV3
      (Variables|Default|SetItemCode "Item_Armor_C_01_Lv3_C")
      (Components|StaticMesh|SetStaticMesh _staticmesh "/Game/Vest/LV3/LightVest_LV3.LightVest_LV3"))))

(fn ConstructionScript)