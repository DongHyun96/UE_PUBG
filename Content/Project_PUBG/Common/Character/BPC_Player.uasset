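; Player character Blueprint for a PUBG-style project, mainly handling death, with empty Tick and BeginPlay.
; The Death event zeroes mesh velocities, switches to ragdoll physics and disables player 0's input.
; A debug B key hides the HUD, stops ticking, calls CharacterDead and disables input.
; Overlap prints camera active state; unconnected trace, unpossess and debug nodes remain, and a note marks F-key interaction as in preparation.
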(event Custom|Death
  (bind _mesh (Variables|Character|GetMesh))
  (bind _mesh_2 (Variables|Character|GetMesh))
  (Physics|SetPhysicsLinearVelocity _mesh_2 "0, 0, 0" false "None")
  (Class|PrimitiveComponent|SetPhysicsAngularVelocityinDegrees _mesh_2 "0, 0, 0" false "None")
  (Physics|SetSimulatePhysics _mesh true)
  (Collision|SetCollisionProfileName _mesh "Ragdoll" true :!class /Script/Engine.PrimitiveComponent)
  (Class|SkeletalMeshComponent|SetAllBodiesBelowSimulatePhysics (Variables|Character|GetMesh) (Utilities|String|StringToName (Utilities|String|ToString(Text) (Utilities|Text|ToText(Name) "Spine"))) true true)
  (Collision|SetCollisionEnabled _mesh "QueryAndPhysics")
  (Input|DisableInput (Game|GetPlayerController 0)))

(event EventBeginPlay)

(event Collision|EventActorBeginOverlap
  (params (OtherActor :type Actor%20Object%20Reference))
  (Development|PrintString (Utilities|String|ToString(Boolean) (Components|Activation|IsActive (Variables|Components|GetCamera)))))

(event EventTick
  (params (DeltaSeconds :type Float%20%28single-precision%29))
  ;[1 1 1] F Key Interaction 준비중.
)

(event Input|KeyboardEvents|DebugKeyB
  (params (Key :type Key%20Structure :default "None") (ActionValue :type Input%20Action%20Value%20Structure))
  (:Pressed
    (Widget|SetVisibility (Variables|Default|GetHUDWidget) "Collapsed")
    (Actor|Tick|SetActorTickEnabled false)
    (Class|CBasicCharacter|CharacterDead)
    (Input|DisableInput (Game|GetPlayerController 0))))

(fn ConstructionScript)