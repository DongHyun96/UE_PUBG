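; Spectator enemy character Blueprint that supplies HP bar and reload audio hooks.
; On BeginPlay it casts the HPBarWidget's user widget to C_EnemyHPWidget and caches it as EnemyHPBarWidget.
; Two events stop the bullet and magazine reload sounds after a short delay if they are playing.
; Tick is empty, and a node that would rotate toward the player camera is left unconnected.
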(event EventBeginPlay
  (bind _asc_enemy_hpwidget (Utilities|Casting|CastToC_EnemyHPWidget (UserInterface|GetUserWidgetObject (Variables|Default|GetHPBarWidget))))
  (Variables|Default|SetEnemyHPBarWidget _asc_enemy_hpwidget))

(event EventTick
  (params (DeltaSeconds :type Float%20%28single-precision%29)))

(event EventStopReloadBulletSound
  (bind _reloadbulletaudiocomp (Variables|Default|GetReloadBulletAudioComp))
  ;[1 1 1] Stop Reload Sound
  (Utilities|IsValid _reloadbulletaudiocomp
    (:Is%20Valid
      (if (Audio|Components|Audio|IsPlaying _reloadbulletaudiocomp)
        (Audio|Components|Audio|StopDelayed _reloadbulletaudiocomp 0.1)))))

(event EventStopReloadMagazineSound
  (bind _reloadmagazineaudiocomp (Variables|Default|GetReloadMagazineAudioComp))
  ;[1 1 1] Stop Reload Sound
  (Utilities|IsValid _reloadmagazineaudiocomp
    (:Is%20Valid
      (if (Audio|Components|Audio|IsPlaying _reloadmagazineaudiocomp)
        (Audio|Components|Audio|StopDelayed _reloadmagazineaudiocomp 0.1)))))

(fn ConstructionScript)