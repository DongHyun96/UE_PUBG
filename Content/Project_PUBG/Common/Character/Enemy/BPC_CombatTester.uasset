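; Combat tester enemy character that shows HP, boost and AI debug info through widget components.
; BeginPlay caches the HP and boost bars from the HP widget, and Tick turns the target-name widget toward the player camera.
; Events push target name, sight-range character names and stun time into that widget.
; Two other events stop the bullet and magazine reload sounds after a short delay.
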(event EventBeginPlay
  (Development|PrintString "BeginPlay" true true "(R=0.000000,G=0.660000,B=1.000000,A=1.000000)" 2e+01)
  (bind _aswbp_enemy_hpwidget (Utilities|Casting|CastToWBP_EnemyHPWidget (UserInterface|GetUserWidgetObject (Variables|Default|GetHPBarWidget))))
  (Variables|Default|SetHPBar (Variables|/Game/Project_PUBG/DongHyun/Character/Widget/EnemyWidget/WBP_EnemyHPWidget.WBP_EnemyHPWidget_C|GetHPBar _aswbp_enemy_hpwidget))
  (Variables|Default|SetBoostBar (Variables|/Game/Project_PUBG/DongHyun/Character/Widget/EnemyWidget/WBP_EnemyHPWidget.WBP_EnemyHPWidget_C|GetBoostBar _aswbp_enemy_hpwidget)))

(event EventTick
  (params (DeltaSeconds :type Float%20%28single-precision%29))
  (Transformation|SetWorldRotation (Variables|Default|GetTargetCharacterNameWidget) (Class|KismetMathLibrary|QuatRotator (Math|Conversions|ToQuaternion(Rotator) (- (Camera|GetCameraLocation (Variables|/Script/Engine.PlayerController|GetPlayerCameraManager (Game|GetPlayerController 0))) (Transformation|GetWorldLocation (Variables|Default|GetTargetCharacterNameWidget))))) false false))

(event EventSetTargetCharacterWidgetName
  (params (TargetCharacterName :type String))
  (bind _aswbp_enemy_target_character (Utilities|Casting|CastToWBP_EnemyTargetCharacter (UserInterface|GetWidget (Variables|Default|GetTargetCharacterNameWidget))))
  (Default|InitTargetCharacterName _aswbp_enemy_target_character TargetCharacterName))

(event EventSetSightRangeCharactersName
  (params (SightRangeLevel :type ESightRangeLevel%20Enum :default "Level1") (SightRangeCharactersName :type String))
  (bind _aswbp_enemy_target_character (Utilities|Casting|CastToWBP_EnemyTargetCharacter (UserInterface|GetWidget (Variables|Default|GetTargetCharacterNameWidget))))
  (Default|InitLevelCharacterNames _aswbp_enemy_target_character SightRangeLevel SightRangeCharactersName))

(event EventSetStunnedTime
  (params (Time :type Float%20%28single-precision%29))
  (bind _aswbp_enemy_target_character (Utilities|Casting|CastToWBP_EnemyTargetCharacter (UserInterface|GetWidget (Variables|Default|GetTargetCharacterNameWidget))))
  (Default|InitStunnedTime _aswbp_enemy_target_character Time))

(event EventStopReloadBulletSound
  (bind _reloadbulletaudiocomp (Variables|Default|GetReloadBulletAudioComp))
  ;[1 1 1] Stop Reload Sound
  (Utilities|IsValid _reloadbulletaudiocomp
    (:Is%20Valid
      (if (Audio|Components|Audio|IsPlaying _reloadbulletaudiocomp)
        (Audio|Components|Audio|StopDelayed _reloadbulletaudiocomp 0.1)))))

(event EventStopReloadMagazineSound
  (bind _reloadmagazineaudiocomp (Variables|Default|GetReloadMagazineAudioComp))
  ;[1 1 1] Stop Reload Sound
  (Utilities|IsValid _reloadmagazineaudiocomp
    (:Is%20Valid
      (if (Audio|Components|Audio|IsPlaying _reloadmagazineaudiocomp)
        (Audio|Components|Audio|StopDelayed _reloadmagazineaudiocomp 0.1)))))

(fn ConstructionScript)