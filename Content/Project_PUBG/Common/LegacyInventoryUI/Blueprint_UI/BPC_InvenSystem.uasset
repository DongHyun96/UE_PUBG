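; Inventory component for the player character that picks up backpacks from the world.
; IA_F sphere-traces from the follow camera; a hit BP_BackPack has its item data added to BackPackSlot and is destroyed.
; Logic to toggle the equipment UI, cursor, input mode and movement exists but is disconnected, so IA_I does nothing.
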(event Input|EnhancedActionEvents|EnhancedInputActionIA_I
  (params (ActionValue :type Boolean) (ElapsedSeconds :type Float%20%28double-precision%29) (TriggeredSeconds :type Float%20%28double-precision%29) (InputAction :type Input%20Action%20Object%20Reference :default "/Game/Project_PUBG/Common/Character/Input/IA_I.IA_I"))
  ;[1 1 1] InvenSystem Panel
)

(event Input|EnhancedActionEvents|EnhancedInputActionIA_F
  (params (ActionValue :type Boolean) (ElapsedSeconds :type Float%20%28double-precision%29) (TriggeredSeconds :type Float%20%28double-precision%29) (InputAction :type Input%20Action%20Object%20Reference :default "/Game/Project_PUBG/Common/Character/Input/IA_F.IA_F"))
  (bind _follow_camera (Variables|Default|GetFollow%20Camera))
  (bind _returnvalue (Transformation|GetWorldLocation _follow_camera))
  (bind _outhit (Collision|SphereTraceForObjects _returnvalue (+ _returnvalue (* (Math|Vector|GetForwardVector (Transformation|GetWorldRotation _follow_camera)) 1000)) 15.0 (Utilities|Array|MakeArray "ObjectTypeQuery2") false 0 "ForDuration"))
  (if true
    (bind _asbp_back_pack (Utilities|Casting|CastToBP_BackPack (.HitActor (Collision|BreakHitResult _outhit))))
    (CallFunction|AddBackPack (Variables|/Game/Project_PUBG/Common/LegacyInventoryUI/Blueprint_UI/Test/BP_BackPack.BP_BackPack_C|GetItem%20Data _asbp_back_pack))
    (Actor|DestroyActor _asbp_back_pack)
    (Development|PrintString "Get item")))

(event EventBeginPlay
  (bind _asbpc_player (Utilities|Casting|CastToBPC_Player (Components|GetOwner)))
  (Variables|Default|SetFollow%20Camera (Variables|/Game/Project_PUBG/Common/Character/BPC_Player.BPC_Player_C|GetCamera _asbpc_player)))

(fn AddBackPack
  (params (NewBackPack :type S%20Slots%20Structure%20%28by%20ref%29))
  (Utilities|Array|Add (Variables|Default|GetBackPackSlot) NewBackPack))