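; Bullet decal actor for gun weapons that removes itself a few seconds after it spawns.
; BeginPlay sets a fixed lifetime, which Tick counts down by delta time before destroying the actor once it runs out.
; The overlap event is disabled, the construction script is empty, and a leftover debug print never runs.
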(event EventBeginPlay
  (Variables|Default|SetLifeTime 5.0))

(event Collision|EventActorBeginOverlap
  (params (OtherActor :type Actor%20Object%20Reference)))

(event EventTick
  (params (DeltaSeconds :type Float%20%28single-precision%29))
  (Variables|Default|SetLifeTime (- (Variables|Default|GetLifeTime) DeltaSeconds))
  (if (<= (Variables|Default|GetLifeTime) 0.0)
    (Actor|DestroyActor)))

(fn ConstructionScript)