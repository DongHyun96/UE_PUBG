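; BPC_Player is a player character Blueprint that pushes its current health to the player HUD.
; UpdateHPonHUD casts the HUD component's widget to WBP_PlayerHUD and passes it the current HP from the stat component.
; BeginPlay, Tick, overlap and the construction script are empty, leaving only unconnected debug nodes for camera, spring arm and head bone positions.
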(event EventBeginPlay)

(event Collision|EventActorBeginOverlap
  (params (OtherActor :type Actor%20Object%20Reference)))

(event EventTick
  (params (DeltaSeconds :type Float%20%28single-precision%29)))

(event EventUpdateHPonHUD
  (bind _aswbp_player_hud (Utilities|Casting|CastToWBP_PlayerHUD (Variables|/Script/UE_PUBG.C_HUDComponent|GetHUDWidget (Variables|Default|GetHUDComponent))))
  (Default|OnUpdateHP _aswbp_player_hud (Class|CStatComponent|GetCurHP (Variables|Default|GetStatComponent))))

(fn ConstructionScript)