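; Custom nav link proxy Blueprint that handles AI agents reaching its smart link in a PUBG-style project.
; On BeginPlay, two flags independently control whether the left and right point spheres move to the world locations returned for their link points.
; When an agent reaches the smart link, it passes the agent and destination to OnReceiveSmartLinkReached, whose logic lives outside this graph.
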(event EventBeginPlay
  (if (Variables|Default|GetbAdjustLeftPointToNearestNavLinkProxyPoint)
    (Transformation|SetWorldLocation (Variables|Default|GetLeftPointSphere) (Class|CCustomNavLinkProxy|GetLeftPointWorldLocation) false false))
  (if (Variables|Default|GetbAdjustRightPointToNearestNavLinkProxyPoint)
    (Transformation|SetWorldLocation (Variables|Default|GetRightPointSphere) (Class|CCustomNavLinkProxy|GetRightPointWorldLocation) false false)))

(event Collision|EventActorBeginOverlap
  (params (OtherActor :type Actor%20Object%20Reference)))

(event EventTick
  (params (DeltaSeconds :type Float%20%28single-precision%29)))

(event EventSmartLinkReached
  (params (Agent :type Actor%20Object%20Reference) (Destination :type Vector%20%28by%20ref%29 :default "0, 0, 0"))
  (Class|CCustomNavLinkProxy|OnReceiveSmartLinkReached Agent Destination))

(fn ConstructionScript)