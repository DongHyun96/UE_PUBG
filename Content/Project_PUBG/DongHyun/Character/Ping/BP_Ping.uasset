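; BP_Ping is a ping marker actor that shows a widget at its location and resizes it by camera distance.
; Every Tick it measures the distance to the player camera and sets the widget's render scale in linear proportion, so it grows as the camera moves away.
; Beyond a fixed cutoff distance it sets the scale to zero, which hides the marker.
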(event EventBeginPlay)

(event Collision|EventActorBeginOverlap
  (params (OtherActor :type Actor%20Object%20Reference)))

(event EventTick
  (params (DeltaSeconds :type Float%20%28single-precision%29))
  (bind _returnvalue (Game|GetPlayerCameraManager 0))
  (bind _returnvalue_2 (Transformation|GetActorLocation))
  (bind _returnvalue_3 (Camera|GetCameraLocation _returnvalue))
  (bind _returnvalue_4 (Math|Vector|Distance(Vector) _returnvalue_2 _returnvalue_3))
  (if (> _returnvalue_4 5e+04)
    (Widget|Transform|SetRenderScale (UserInterface|GetUserWidgetObject (Variables|Default|GetWidget)) "(X=0.000000,Y=0.000000)")
    (else
      (Widget|Transform|SetRenderScale (UserInterface|GetUserWidgetObject (Variables|Default|GetWidget)) (Math|Conversions|ToVector2D(Vector) (* _returnvalue_4 2e-05))))))

(fn ConstructionScript)