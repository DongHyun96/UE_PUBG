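; Airplane actor Blueprint that plays looping C-130 military cargo plane engine audio.
; BeginPlay keeps the Audio component silent until StartEngineSound plays it and also spawns the C-130 sound attached to it.
; OnAudioFinished repeats both actions to loop the audio.
; StopEngineSound stops only the Audio component, as the spawned sounds are not stored.
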(event OnAudioFinished(Audio)
  (bind _audio (Variables|Default|GetAudio))
  (Audio|Components|Audio|Play _audio 0.0)
  (Audio|SpawnSoundAttached "/Game/Project_PUBG/Common/Sounds/Aripalne/PUBG_Mobile_C_130_Military_Cargo_Plane_Sound_Effect.PUBG_Mobile_C_130_Military_Cargo_Plane_Sound_Effect" _audio "None" "0, 0, 0" "0, 0, 0" "KeepRelativeOffset" false 1.0 1.0 0.0 0 0))

(event EventBeginPlay
  (Audio|Components|Audio|Stop (Variables|Default|GetAudio)))

(event Collision|EventActorBeginOverlap
  (params (OtherActor :type Actor%20Object%20Reference)))

(event EventTick
  (params (DeltaSeconds :type Float%20%28single-precision%29)))

(event EventStartEngineSound
  (bind _audio (Variables|Default|GetAudio))
  (Audio|Components|Audio|Play _audio 0.0)
  (Audio|SpawnSoundAttached "/Game/Project_PUBG/Common/Sounds/Aripalne/PUBG_Mobile_C_130_Military_Cargo_Plane_Sound_Effect.PUBG_Mobile_C_130_Military_Cargo_Plane_Sound_Effect" _audio "None" "0, 0, 0" "0, 0, 0" "KeepRelativeOffset" false 1.0 1.0 0.0 0 0))

(event EventStopEngineSound
  (Audio|Components|Audio|Stop (Variables|Default|GetAudio)))

(fn ConstructionScript)